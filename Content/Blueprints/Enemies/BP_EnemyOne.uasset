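; BP_EnemyOne is an enemy that automatically fires projectiles at a steady interval.
; Tick feeds a Delay of FireRate, which ignores calls while pending and so works as a repeating fire timer.
; Each shot spawns a BP_ProjectileEnemy at the ProjectileSpawn transform with fixed damage, velocity along negative Y and scale, then plays EnemyShot at the world origin.
; BeginPlay and the construction script only call their parents.
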(event `self.ReceiveBeginPlay`
  (`parent.ReceiveBeginPlay`))

(event `self.ReceiveTick`
  (params (DeltaSeconds :type "Float (single-precision)"))
  (`parent.ReceiveTick` DeltaSeconds)
  (`KismetSystemLibrary.Delay` (`self.FireRate`))
  (`|SpawnActorFromClass` "/Game/Blueprints/Projectiles/BP_ProjectileEnemy.BP_ProjectileEnemy_C" (`SceneComponent.K2_GetComponentToWorld` (`self.ProjectileSpawn`)) "Undefined" "OverrideRootScale" null 10.0 (0.0 -2000.0 0.0) (2.0 2.0 2.0) null)
  (`GameplayStatics.PlaySoundAtLocation` "/Game/Audio/EnemyShot.EnemyShot"))

(fn `UserConstructionScript`
  (`parent.UserConstructionScript`))