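; Player rocket projectile Blueprint with homing logic that targets the first BP_Player to overlap its HomingBox.
; That player is stored in TEMPORARYVAR and is not replaced while valid.
; Each Tick lerps ProjectileMovement velocity toward the target direction at IncreasedSpeed and sets it as local-space velocity.
; The lerp alpha is zero, so the homing direction currently contributes nothing to the result.
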(event `self.ReceiveTick`
  (params (DeltaSeconds :type "Float (single-precision)"))
  (`/Engine/EditorBlueprintResources/StandardMacros.IsValid` (`self.TEMPORARYVAR`)
    (:`Is Valid`
      (`ProjectileMovementComponent.SetVelocityInLocalSpace` (`self.ProjectileMovement`) (`KismetMathLibrary.VLerp` (`MovementComponent.Velocity` (`self.ProjectileMovement`)) (* (`KismetMathLibrary.Normal` (- (`self.K2_GetActorLocation` (`self.TEMPORARYVAR`)) (`self.K2_GetActorLocation`))) (`self.IncreasedSpeed`)))))))

(event `self.HomingBox.OnComponentBeginOverlap`
  (params (OverlappedComponent :type "PrimitiveComponent Object Reference") (OtherActor :type "Actor Object Reference") (OtherComp :type "PrimitiveComponent Object Reference") (OtherBodyIndex :type Integer) (bFromSweep :type Boolean) (SweepResult :type "HitResult Structure (by ref)"))
  (bind _asbp_player (cast `/Game/Blueprints/BP_Player` OtherActor))
  (`/Engine/EditorBlueprintResources/StandardMacros.IsValid` (`self.TEMPORARYVAR`)
    (:`Is Not Valid`
      (set `self.TEMPORARYVAR` _asbp_player))))

(fn `UserConstructionScript`
  (`parent.UserConstructionScript`))