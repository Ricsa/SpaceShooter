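; BP_ProjectileEnemy is an enemy projectile that damages the player on impact.
; It moves itself each tick with a swept local offset and destroys itself when the game mode's current widget is the replay menu.
; Any mesh hit destroys it; a player hit also applies damage, spawns a hit particle and triggers a camera shake through BP_GameMode.
; The construction script sets its actor scale from a variable.
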(event `self.ReceiveBeginPlay`
  ;[1 1 1] SET GAMEMODE
  (bind _asbp_game_mode (cast `/Game/Blueprints/Misc/BP_GameMode` (`GameplayStatics.GetGameMode`)))
  (set `self.BP_GameModeReference` _asbp_game_mode))

(event `self.ReceiveTick`
  (params (DeltaSeconds :type "Float (single-precision)"))
  ;[1 1 1] MOVE PROJECTILE
  (`self.K2_AddActorLocalOffset` (* (`self.Speed`) DeltaSeconds) true)
  (if (== (`/Game/Blueprints/Misc/BP_GameMode.CurrentWidget` (`self.BP_GameModeReference`)) "/Game/Blueprints/UI/WBP_ReplayMenu.WBP_ReplayMenu_C")
    (`self.K2_DestroyActor`)))

(event `self.ProjectileMesh.OnComponentHit`
  (params (HitComponent :type "PrimitiveComponent Object Reference") (OtherActor :type "Actor Object Reference") (OtherComp :type "PrimitiveComponent Object Reference") (NormalImpulse :type "Vector Structure") (Hit :type "HitResult Structure (by ref)"))
  ;[1 1 1] COLLISION EVENTS
  (bind _asbp_player (cast `/Game/Blueprints/Misc/BP_Player` OtherActor)
    (:`then`
      (`GameplayStatics.ApplyDamage` _asbp_player (`self.Damage`))
      (`GameplayStatics.SpawnEmitterAtLocation` "/Game/Art/Particles/PS_HitPlayer.PS_HitPlayer" (`self.K2_GetActorLocation`))
      (bind _asbp_game_mode (cast `/Game/Blueprints/Misc/BP_GameMode` (`GameplayStatics.GetGameMode`)))
      (`/Game/Blueprints/Misc/BP_GameMode.CallCamShake` _asbp_game_mode "/Game/Blueprints/Misc/BP_CamShakeCollision.BP_CamShakeCollision_C"))
    (:`CastFailed`
      _))
  (`self.K2_DestroyActor`))

(fn `UserConstructionScript`
  (`self.SetActorScale3D` (`self.Scale`)))