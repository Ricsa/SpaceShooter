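; BP_FloatingIsland is a decorative-style island actor that drifts along negative Y and recycles itself once past an offscreen limit.
; The construction script places random tree meshes at three arrow markers, randomizes scale per axis and sets a fixed tilt.
; Tick moves it a fixed step per frame, not scaled by delta time.
; Past the limit, it waits a random delay, has BP_GameMode spawn another island, then destroys itself.
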(event `self.ReceiveTick`
  (params (DeltaSeconds :type "Float (single-precision)"))
  (bind (_returnvalue_x _returnvalue_y) (`KismetMathLibrary.BreakVector` (`SceneComponent.K2_GetComponentLocation` (`self.Scene`))))
  (if (< _returnvalue_y (`self.OffscreenLeft`))
    (`KismetSystemLibrary.Delay` (`KismetMathLibrary.RandomFloatInRange` 1.0 20.0))
    (bind _asbp_game_mode (cast `/Game/Blueprints/Misc/BP_GameMode` (`GameplayStatics.GetGameMode`)))
    (`/Game/Blueprints/Misc/BP_GameMode.SpawnIsland` _asbp_game_mode)
    (`self.K2_DestroyActor`)
    (else
      (`SceneComponent.K2_AddWorldOffset` (`self.Scene`) (0.0 -20.0 0.0) false false))))

(fn `SetSpawnPoints`
  (set `self.SpawnPoints` (`|MakeArray` (`SceneComponent.GetRelativeTransform` (`self.Arrow`)) (`SceneComponent.GetRelativeTransform` (`self.Arrow1`)) (`SceneComponent.GetRelativeTransform` (`self.Arrow2`)))))

(fn `SpawnTrees`
  (bind _trees (`self.Trees`))
  (bind _spawnpoints (`self.SpawnPoints`))
  (for _index (range (+ (`KismetArrayLibrary.Array_LastIndex` _spawnpoints) 1))
    (bind _returnvalue (`AddComponent|NODE_AddStaticMeshComponent-0` :`RelativeTransform` (`|GetArrayItem` _spawnpoints _index)))
    (`StaticMeshComponent.SetStaticMesh` _returnvalue (`|GetArrayItem` _trees (`KismetMathLibrary.RandomIntegerInRange` 0 (`KismetArrayLibrary.Array_LastIndex` _trees))))))

(fn `UserConstructionScript`
  (bind _returnvalue (`KismetMathLibrary.RandomFloatInRange` 0.3 1.0))
  (`self.SetSpawnPoints`)
  (`self.SpawnTrees`)
  (`self.SetActorScale3D` (`KismetMathLibrary.MakeVector` _returnvalue _returnvalue _returnvalue))
  (`self.K2_SetActorRotation` (struct :`Pitch` 15.0 :`Yaw` -50.0 :`Roll` -15.0)))